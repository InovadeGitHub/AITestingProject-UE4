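; Player inventory component that holds an array of item actors and tracks a selected slot.
; Every tick it refreshes visibility so only the valid item in the selected slot is shown and all others are hidden in game.
; Helper functions return the currently selected item and report whether the inventory holds any entries.
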(event `self.ReceiveTick`
  (params (DeltaSeconds :type "Float (single-precision)"))
  (`self.Refresh Inventory`))

(fn `Get Currently Selected Item`
  (returns (ReturnValue :type "/Game/Blueprints/Objects/BP_BaseItem Object Reference"))
  (return (`|GetArrayItem` (`self.Inventory`) (`self.Selected Inventory Slot`))))

(fn `Has Item`
  (returns (ReturnValue :type Boolean))
  (return (> (`KismetArrayLibrary.Array_Length` (`self.Inventory`)) 0)))

(fn `Refresh Inventory`
  (for (_array_element _array_index) (`self.Inventory`)
    (`/Engine/EditorBlueprintResources/StandardMacros.IsValid` _array_element
      (:`Is Valid`
        (`Actor.SetActorHiddenInGame` _array_element (!= _array_index (`self.Selected Inventory Slot`)))))))