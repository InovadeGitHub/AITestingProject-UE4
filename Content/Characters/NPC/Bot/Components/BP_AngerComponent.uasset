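; Bot component that builds an anger value while the player is inside the bot's personal space.
; Looping timers re-bind the bot's enter and leave events, the enter binding only while it moves; entering starts a timer that adds clamped anger.
; Maximum anger triggers FullyAngry and clears all timers.
; Leaving stops the buildup without lowering anger and fires a dispatcher, re-bound on Tick, that restarts the movement check.
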(event `self.ReceiveBeginPlay`
  (bind _asbp_bot (cast `/Game/Characters/NPC/Bot/BP_Bot` (`self.GetOwner`)))
  (set `self.Bot` _asbp_bot)
  (bind _returnvalue (`KismetSystemLibrary.K2_SetTimer` null "Check Anger" 2.0 true))
  (set `self.Check Anger Timer` _returnvalue)
  (bind _returnvalue_2 (`KismetSystemLibrary.K2_SetTimer` null "Did Player Leave" 0.01 true))
  (set `self.Did Player Leave Timer` _returnvalue_2))

(event `Check Anger`
  (bind _bot (`self.Bot`))
  (if (`/Game/Characters/NPC/Bot/BP_Bot.bMoving` _bot)
    (add `/Game/Characters/NPC/Bot/BP_Bot.PlayerEnteredPersonalSpace` _bot (delegate `In Space`))))

(event `Did Player Leave`
  (add `/Game/Characters/NPC/Bot/BP_Bot.PlayerLeftPersonalSpace` (`self.Bot`) (`|CreateDelegate` :!event `Player Left Personal Space`)))

(event `In Space`
  (bind _returnvalue (`KismetSystemLibrary.K2_SetTimer` null "Player Entered Personal Space" 0.5 true))
  (set `self.Player Entered` _returnvalue))

(event `self.ReceiveTick`
  (params (DeltaSeconds :type "Float (single-precision)"))
  (add `self.CheckAngerTimerCleared` (delegate `Restart Check Anger Timer`)))

(event `Restart Check Anger Timer`
  (bind _returnvalue (`KismetSystemLibrary.K2_SetTimer` null "Check Anger" 2.0 true))
  (set `self.Check Anger Timer` _returnvalue))

(fn `Add Anger`
  (params (`Anger To Add` :type "Float (double-precision)"))
  (set `self.Anger` (`KismetMathLibrary.FClamp` (+ (`self.Anger`) `Anger To Add`) 0.0 100.0)))

(fn `Player Entered Personal Space`
  (`self.Add Anger` 25.0)
  (if (>= (`self.Anger`) 100.0)
    (`/Game/Characters/NPC/Bot/BP_Bot.Fully Angry` (`self.Bot`))
    (`KismetSystemLibrary.K2_ClearAndInvalidateTimerHandle` (`self.Did Player Leave Timer`))
    (`KismetSystemLibrary.K2_ClearAndInvalidateTimerHandle` (`self.Player Entered`))
    (`KismetSystemLibrary.K2_ClearAndInvalidateTimerHandle` (`self.Check Anger Timer`))))

(fn `Player Left Personal Space`
  (`KismetSystemLibrary.K2_ClearAndInvalidateTimerHandle` (`self.Player Entered`))
  (`KismetSystemLibrary.K2_ClearAndInvalidateTimerHandle` (`self.Check Anger Timer`))
  (`self.CheckAngerTimerCleared`))

(fn `Subtract Anger`
  (params (`Anger To Subtract` :type "Float (double-precision)"))
  (set `self.Anger` (`KismetMathLibrary.FClamp` (- (`self.Anger`) `Anger To Subtract`) 0.0 100.0)))