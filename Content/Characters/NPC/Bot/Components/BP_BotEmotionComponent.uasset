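; Emotion component for BP_Bot that tracks clamped Anger and Happiness, mirroring them to blackboard keys and, each tick, to mesh material parameters.
; A fast looping timer repeatedly binds the personal-space event; intrusions add anger, switching bot state at maximum.
; Another timer sphere-traces for a pumpkin pie in the player's inventory, then flags the blackboard, changes state and stops.
; Adding happiness also lowers anger, without clamping it.
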(event `self.ReceiveBeginPlay`
  (`|ExecutionSequence`
    (:`then_0`
      (bind _asbp_bot (cast `/Game/Characters/NPC/Bot/BP_Bot` (`self.GetOwner`)))
      (set `self.Bot` _asbp_bot))
    (:`then_1`
      (bind _returnvalue (`KismetSystemLibrary.K2_SetTimer` null "Is Player In Personal Space" 0.01 true))
      (set `self.Check Personal Space Timer` _returnvalue))
    (:`then_2`
      (bind _returnvalue_2 (`KismetSystemLibrary.K2_SetTimer` null "Check For Pumpkin Pie" 0.01 true))
      (set `self.Check For Pumpkin Pie Timer` _returnvalue_2))))

(event `self.ReceiveTick`
  (params (DeltaSeconds :type "Float (single-precision)"))
  (bind _staticmesh (`/Game/Characters/NPC/Bot/BP_Bot.StaticMesh` (`self.Bot`)))
  (`MeshComponent.SetScalarParameterValueOnMaterials` _staticmesh "Anger" (`self.Remap Anger`))
  (`MeshComponent.SetScalarParameterValueOnMaterials` _staticmesh "Happiness" (`self.Remap Happiness`)))

(event `Is Player In Personal Space`
  ;[1 0.05208 0.05208] Check Personal Space
  (add `/Game/Characters/NPC/Bot/BP_Bot.Player Entered Personal Space` (`self.Bot`) (`|CreateDelegate` :!event `Player Inside Personal Space`)))

(event `Check For Pumpkin Pie`
  (bind _bot (`self.Bot`))
  (bind _returnvalue (`Actor.K2_GetActorLocation` (`self.Bot`)))
  (bind (_outhit _returnvalue_2) (`KismetSystemLibrary.SphereTraceSingle` _returnvalue _returnvalue 500.0 "TraceTypeQuery1"))
  (if _returnvalue_2
    (bind _asbp_pumpkin_pie (cast `/Game/Blueprints/Objects/BP_PumpkinPie` (`.HitActor` (`GameplayStatics.BreakHitResult` _outhit))))
    (if (`KismetArrayLibrary.Array_Contains` (`/Game/Characters/Player/Components/BP_InventoryComponent.Inventory` (`/Game/Characters/Player/BP_Player.InventoryComponent` (`/Game/GameplayLogic/FunctionLibrary/BP_FunctionLibrary.Get Player`))) _asbp_pumpkin_pie)
      (`/Game/Characters/NPC/Bot/BP_Bot.Set Blackboard Key Value` _bot "NewEnumerator0" "bPumpkinPieDetected" true (0.0 0.0 0.0) null 0 0.0)
      (`/Game/Characters/NPC/Bot/BP_Bot.Set Bot State` _bot "NewEnumerator3")
      (`KismetSystemLibrary.K2_ClearAndInvalidateTimerHandle` (`self.Check For Pumpkin Pie Timer`)))))

(fn `Add Anger`
  (params (`Anger To Add` :type "Float (double-precision)"))
  (returns (ReturnValue :type "Float (double-precision)"))
  (bind _output_get (set `self.Anger` (`KismetMathLibrary.FClamp` (+ (`self.Anger`) `Anger To Add`) 0.0 100.0)))
  (`/Game/Characters/NPC/Bot/BP_Bot.Set Blackboard Key Value` (`self.Bot`) "NewEnumerator5" "Anger" false (0.0 0.0 0.0) null 0 _output_get)
  (return _output_get))

(fn `Add Happiness`
  (params (`Happiness To Add` :type "Float (double-precision)"))
  (returns (ReturnValue :type "Float (double-precision)"))
  (bind _bot (`self.Bot`))
  (bind _output_get (set `self.Happiness` (`KismetMathLibrary.FClamp` (+ (`self.Happiness`) `Happiness To Add`) 0.0 100.0)))
  (bind _output_get_2 (set `self.Anger` (- (`self.Anger`) `Happiness To Add`)))
  (`/Game/Characters/NPC/Bot/BP_Bot.Set Blackboard Key Value` _bot "NewEnumerator5" "Happiness" false (0.0 0.0 0.0) null 0 _output_get)
  (`/Game/Characters/NPC/Bot/BP_Bot.Set Blackboard Key Value` _bot "NewEnumerator5" "Anger" false (0.0 0.0 0.0) null 0 _output_get_2)
  (return _output_get))

(fn `Player Inside Personal Space`
  (`KismetSystemLibrary.PrintString` "You are in my personal space." true true (struct :`R` 1.0 :`A` 1.0))
  (bind _returnvalue (`self.Add Anger` 25.0))
  (`self.Print Anger` _returnvalue)
  (if (>= _returnvalue 100.0)
    (`/Game/Characters/NPC/Bot/BP_Bot.Set Bot State` (`self.Bot`) "NewEnumerator2")))

(fn `Print Anger`
  (params (Anger :type "Float (double-precision)"))
  (`KismetSystemLibrary.PrintString` (`KismetStringLibrary.Concat_StrStr` "Current Anger: " (`KismetStringLibrary.Conv_DoubleToString` Anger)) true true (struct :`R` 1.0 :`A` 1.0)))

(fn `Print Happiness`
  (params (Happiness :type "Float (double-precision)"))
  (`KismetSystemLibrary.PrintString` (`KismetStringLibrary.Concat_StrStr` "Current Happiness: " (`KismetStringLibrary.Conv_DoubleToString` Happiness)) true true (struct :`G` 0.999998 :`A` 1.0)))

(fn `Remap Anger`
  (returns (ReturnValue :type "Float (double-precision)"))
  (return (`KismetMathLibrary.MapRangeClamped` (`self.Anger`) 0.0 100.0 0.0 1.0)))

(fn `Remap Happiness`
  (returns (ReturnValue :type "Float (double-precision)"))
  (return (`KismetMathLibrary.MapRangeClamped` (`self.Happiness`) 0.0 100.0 0.0 1.0)))

(fn `Subtract Anger`
  (params (`Anger To Subtract` :type "Float (double-precision)"))
  (returns (ReturnValue :type "Float (double-precision)"))
  (bind _output_get (set `self.Anger` (`KismetMathLibrary.FClamp` (- (`self.Anger`) `Anger To Subtract`) 0.0 100.0)))
  (`/Game/Characters/NPC/Bot/BP_Bot.Set Blackboard Key Value` (`self.Bot`) "NewEnumerator5" "Anger" false (0.0 0.0 0.0) null 0 _output_get)
  (return _output_get))

(fn `Subtract Happiness`
  (params (`Happiness To Subtract` :type "Float (double-precision)"))
  (returns (ReturnValue :type "Float (double-precision)"))
  (bind _output_get (set `self.Happiness` (`KismetMathLibrary.FClamp` (- (`self.Happiness`) `Happiness To Subtract`) 0.0 100.0)))
  (`/Game/Characters/NPC/Bot/BP_Bot.Set Blackboard Key Value` (`self.Bot`) "NewEnumerator5" "Happiness" false (0.0 0.0 0.0) null 0 _output_get)
  (return _output_get))