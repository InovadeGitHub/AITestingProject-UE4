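; BP_LocationCube is a prototype cube actor that positions itself between two other cubes and knocks away characters that hit it.
; The construction script moves it to the XY midpoint of FirstCube and SecondCube at a fixed height, provided both references are valid and not itself.
; On Hit, it launches the character away from its center, overriding velocity with a strength scaled unclamped from the character's current speed.
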(event `self.ReceiveHit`
  (params (MyComp :type "PrimitiveComponent Object Reference") (Other :type "Actor Object Reference") (OtherComp :type "PrimitiveComponent Object Reference") (bSelfMoved :type Boolean) (HitLocation :type "Vector Structure") (HitNormal :type "Vector Structure") (NormalImpulse :type "Vector Structure") (Hit :type "HitResult Structure (by ref)"))
  (bind _ascharacter (cast `Character` Other))
  (`Character.LaunchCharacter` _ascharacter (* (`KismetMathLibrary.GetDirectionUnitVector` (`self.K2_GetActorLocation`) (`self.K2_GetActorLocation` _ascharacter)) (`KismetMathLibrary.MapRangeUnclamped` (`KismetMathLibrary.VSize` (`self.GetVelocity` _ascharacter)) 50.0 100.0 500.0 1000.0)) true true))

(fn `UserConstructionScript`
  (bind (_returnvalue_x _returnvalue_y) (`KismetMathLibrary.BreakVector` (/ (+ (`self.K2_GetActorLocation` (`self.First Cube`)) (`self.K2_GetActorLocation` (`self.Second Cube`))) 2.0)))
  (bind _first_cube (`self.First Cube`)
    (:`then`
      (if (not (== _first_cube self))
        (bind _second_cube (`self.Second Cube`)
          (:`then`
            (if (not (== _second_cube self))
              (`self.K2_SetActorLocation` (`KismetMathLibrary.MakeVector` _returnvalue_x _returnvalue_y 300.0))))
          (:`else`))))
    (:`else`)))