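; Prototype physics cube that homes in on the actor referenced by ActorToInheritVelocityFrom.
; Each Tick, if that actor is valid and not itself, it adds a fixed horizontal push toward it to the cube's linear velocity and turns to face it.
; The push accumulates every frame without delta-time scaling, so acceleration depends on frame rate.
; Despite the variable name, only the target's location is read, never its velocity.
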(event `self.ReceiveTick`
  (params (DeltaSeconds :type "Float (single-precision)"))
  (bind _returnvalue (`self.K2_GetActorLocation`))
  (bind _actor_to_inherit_velocity_from (`self.Actor To Inherit Velocity From`)
    (:`then`
      (if (not (== _actor_to_inherit_velocity_from self))
        (bind _returnvalue_2 (`self.K2_GetActorLocation` _actor_to_inherit_velocity_from))
        (bind (_returnvalue_x _returnvalue_y) (`KismetMathLibrary.BreakVector` (* (`KismetMathLibrary.GetDirectionUnitVector` _returnvalue _returnvalue_2) 25.0)))
        (`PrimitiveComponent.SetPhysicsLinearVelocity` (`self.Cube`) (`KismetMathLibrary.MakeVector` _returnvalue_x _returnvalue_y) true "None")
        (`self.K2_SetActorRotation` (`KismetMathLibrary.FindLookAtRotation` _returnvalue _returnvalue_2))))
    (:`else`)))

(fn `UserConstructionScript`)