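; BP_BaseItem is a base item with pickup and drop behavior for its StaticMesh.
; OnPickup turns off physics and collision, while OnDrop restores both and detaches the actor, keeping its world transform.
; An AttachToComponent helper snaps location and rotation to a given parent, keeping world scale.
; Its only call here, targeting the player's DefaultPickupPosition, is unwired, and SetPickupPosition is empty.
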(event `/Game/GameplayLogic/BlueprintInterfaces/BPI_Interaction.OnPickup`
  (bind _staticmesh (`self.StaticMesh`))
  (`PrimitiveComponent.SetSimulatePhysics` _staticmesh false)
  (`PrimitiveComponent.SetCollisionEnabled` _staticmesh "NoCollision"))

(event `/Game/GameplayLogic/BlueprintInterfaces/BPI_Interaction.OnDrop`
  (bind _staticmesh (`self.StaticMesh`))
  (`PrimitiveComponent.SetSimulatePhysics` _staticmesh true)
  (`PrimitiveComponent.SetCollisionEnabled` _staticmesh "QueryAndPhysics")
  (`self.K2_DetachFromActor` "KeepWorld" "KeepWorld" "KeepWorld"))

(fn `Attach To Component`
  (params (Parent :type "SceneComponent Object Reference"))
  (`self.K2_AttachToComponent` Parent "None" "SnapToTarget" "SnapToTarget" "KeepWorld"))

(fn `Set Pickup Position`)

(fn `UserConstructionScript`)