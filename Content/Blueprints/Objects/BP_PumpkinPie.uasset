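; BP_PumpkinPie is a pickup item the player can give to a bot to make it happier.
; On apply, a short line trace finds the bot, and the pie is used only if the bot's blackboard flags it as detected.
; It then leaves the inventory, adds happiness, resets the flag and bot state, starts a looping pie-check timer stored on the EmotionComponent, and destroys itself.
; Its pickup position comes from the player.
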(event `/Game/GameplayLogic/BlueprintInterfaces/BPI_Interaction.OnApply`
  (params (Player :type "/Game/Characters/Player/BP_Player Object Reference"))
  (bind _bot (`self.Bot`))
  (bind _emotioncomponent (`/Game/Characters/NPC/Bot/BP_Bot.EmotionComponent` _bot))
  (bind (_out_hit _returnvalue) (`/Game/Characters/Player/BP_Player.Linetrace` Player 250.0 false))
  (if _returnvalue
    (bind _asbp_bot (cast `/Game/Characters/NPC/Bot/BP_Bot` (`.HitActor` (`GameplayStatics.BreakHitResult` _out_hit))))
    (bind _output_get (set `self.Bot` _asbp_bot))
    (if (`/Game/Characters/NPC/Bot/BP_Bot.Get Blackboard Key Value` _output_get "NewEnumerator0" "bPumpkinPieDetected")
      (`KismetArrayLibrary.Array_RemoveItem` (`/Game/Characters/Player/Components/BP_InventoryComponent.Inventory` (`/Game/Characters/Player/BP_Player.InventoryComponent` Player)) self)
      (bind _returnvalue_2 (`/Game/Characters/NPC/Bot/Components/BP_BotEmotionComponent.Add Happiness` _emotioncomponent 50.0))
      (`/Game/Characters/NPC/Bot/Components/BP_BotEmotionComponent.Print Happiness` _emotioncomponent _returnvalue_2)
      (`/Game/Characters/NPC/Bot/BP_Bot.Set Blackboard Key Value` _bot "NewEnumerator0" "bPumpkinPieDetected" false (0.0 0.0 0.0) null 0 0.0)
      (`/Game/Characters/NPC/Bot/BP_Bot.Set Bot State` _bot "NewEnumerator0")
      (bind _returnvalue_3 (`KismetSystemLibrary.K2_SetTimer` null "Check For Pumpkin Pie" 0.01 true))
      (set `/Game/Characters/NPC/Bot/Components/BP_BotEmotionComponent.Check For Pumpkin Pie Timer` _returnvalue_3 _emotioncomponent)
      (`self.K2_DestroyActor`))))

(fn `Set Pickup Position`
  (set `self.Pickup Position` (`/Game/Characters/Player/BP_Player.Pumpkin Pie Pickup Position` (`/Game/GameplayLogic/FunctionLibrary/BP_FunctionLibrary.Get Player`)))
  (`parent.Set Pickup Position`))

(fn `UserConstructionScript`
  (`parent.UserConstructionScript`))