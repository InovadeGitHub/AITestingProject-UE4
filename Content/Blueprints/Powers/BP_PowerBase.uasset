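; Base Blueprint for power pickups that the player collects by overlapping their box.
; The first BP_Player overlap stores the player, stops the idle scale-pulse timeline and plays a destroy timeline scaling the actor between zero and its saved scale.
; When that finishes, it calls PowerEvent, an empty hook for child powers to override, then destroys itself.
; The pulse timeline has no play call in the graph.
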(event `self.Box.OnComponentBeginOverlap`
  (params (OverlappedComponent :type "PrimitiveComponent Object Reference") (OtherActor :type "Actor Object Reference") (OtherComp :type "PrimitiveComponent Object Reference") (OtherBodyIndex :type Integer) (bFromSweep :type Boolean) (SweepResult :type "HitResult Structure (by ref)"))
  ;[0.1 0.1 0.1] Begin Overlap
  (bind _asbp_player (cast `/Game/Characters/Player/BP_Player` OtherActor))
  (`/Engine/EditorBlueprintResources/StandardMacros.DoOnce` false
    (:`Completed`
      (set `self.Player` _asbp_player)
      (`TimelineComponent.Stop` (`self.TL_Scale`))
      (set `self.Saved Scale` (`self.GetActorScale3D`))
      (bind (_direction _scale) (`Timeline|TL_Destroy`)
        (:`Update`
          (`self.SetActorScale3D` (`KismetMathLibrary.VLerp` (0.0 0.0 0.0) (`self.Saved Scale`) _scale)))
        (:`Finished`
          (`self.Power Event`)
          (`self.K2_DestroyActor`))))))

(fn `Power Event`)

(fn `UserConstructionScript`)