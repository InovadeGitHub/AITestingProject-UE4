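; Blueprint function library of shared gameplay helpers for fetching the player and generating random vectors.
; Get Player casts player character 0 to BP_Player, falls back to the first BP_Player found in the world, and returns it with its location.
; The fallback does not check for an empty result.
; Random Vector In Range rolls each axis independently between the same Min and Max.
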(fn `Get Player`
  (returns (ReturnValue :type "/Game/Characters/Player/BP_Player Object Reference") (`Player Location` :type "Vector Structure"))
  (bind _asbp_player (cast `/Game/Characters/Player/BP_Player` (`GameplayStatics.GetPlayerCharacter` null))
    (:`then`
      (return _asbp_player (`Actor.K2_GetActorLocation` _asbp_player)))
    (:`CastFailed`
      (bind _outactors (`GameplayStatics.GetAllActorsOfClass` null "/Game/Characters/Player/BP_Player.BP_Player_C"))
      (bind _output (`|GetArrayItem` _outactors))
      (return _output (`Actor.K2_GetActorLocation` _output)))))

(fn `Random Vector In Range`
  (params (Min :type "Float (double-precision)") (Max :type "Float (double-precision)"))
  (returns (ReturnValue :type "Vector Structure"))
  (return (`KismetMathLibrary.MakeVector` (`KismetMathLibrary.RandomFloatInRange` Min Max) (`KismetMathLibrary.RandomFloatInRange` Min Max) (`KismetMathLibrary.RandomFloatInRange` Min Max))))